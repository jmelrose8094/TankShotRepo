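; Water obstacle that acts as a lethal hazard for the tank and ends the game on contact.
; When a Tank_BP actor overlaps the Plane component, the tank is destroyed and the GameOver_BP widget is shown with a visible cursor and UI-only input.
; It then sets StopTime on the MyGame game mode.
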(event OnComponentBeginOverlap(Plane)
  (params (OverlappedComponent :type Primitive%20Component%20Object%20Reference) (OtherActor :type Actor%20Object%20Reference) (OtherComp :type Primitive%20Component%20Object%20Reference) (OtherBodyIndex :type Integer) (bFromSweep :type Boolean) (SweepResult :type Hit%20Result%20Structure%20%28by%20ref%29))
  (bind _returnvalue (Game|GetPlayerController 0))
  (if (Utilities|ClassIsChildOf (Utilities|GetClass OtherActor) "/Game/Tank/Tank_BP.Tank_BP_C")
    (Actor|DestroyActor OtherActor)
    (Variables|/Script/Engine.PlayerController|SetbShowMouseCursor _returnvalue true)
    (Input|SetInputModeGameOnly _returnvalue)
    (bind _returnvalue_2 (UserInterface|CreateWidget "/Game/UI/GameOver_BP.GameOver_BP_C" _returnvalue))
    (UserInterface|Viewport|AddtoViewport _returnvalue_2 0)
    (Input|SetInputModeUIOnly (Game|GetPlayerController 0) 0 "DoNotLock")
    (bind _asmy_game (Utilities|Casting|CastToMyGame (Game|GetGameMode)))
    (Variables|/Game/Tank/MyGame.MyGame_C|SetStop_Time _asmy_game true)))

(event EventBeginPlay)

(event Collision|EventActorBeginOverlap
  (params (OtherActor :type Actor%20Object%20Reference)))

(event EventTick
  (params (DeltaSeconds :type Float%20%28single-precision%29)))

(fn ConstructionScript)
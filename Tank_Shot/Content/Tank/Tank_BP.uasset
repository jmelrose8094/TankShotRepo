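; Player-controlled tank pawn that drives forward and back along the control yaw, turns and looks with input axes, and fires projectiles.
; It attaches a default cannon on BeginPlay and replaces it when overlapping incendiary, explosive or sniper power-ups.
; Fire always launches Tank_Projectile_BP along control rotation with a set velocity, taking only the cooldown from the equipped cannon's FireRate.
; Strafing, cannon Shoot and trace-aimed firing logic are left unconnected.
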(event EventBeginPlay
  ;[1 1 1] Takes gun and attaches it to tank gun location scene component
  (bind _returnvalue (Game|SpawnActorfromClass "/Game/Tank/Cannon_BP.Cannon_BP_C" (Math|Conversions|ToTransform(Vector) "0, 0, 0") "Undefined" 0 0))
  (bind _output_get (Variables|Default|SetEquippedGun _returnvalue))
  (Transformation|AttachComponentToComponent _output_get (Variables|Default|GetGunLocation) "None" "SnapToTarget" "SnapToTarget" "KeepRelative" true))

(event Collision|EventActorBeginOverlap
  (params (OtherActor :type Actor%20Object%20Reference))
  (bind _returnvalue (Math|Conversions|ToTransform(Vector) "0, 0, 0"))
  ;[1 1 1] Change barrel on collision with power-up
  (bind _output_get (Variables|Default|SetOverlappingActor OtherActor))
  (if (Utilities|ClassIsChildOf (Utilities|GetClass _output_get) "/Game/Tank/Power-Ups/Inciediary_Power_Up_BP.Inciediary_Power_Up_BP_C")
    (bind _returnvalue_2 (Game|SpawnActorfromClass "/Game/Tank/Incendiary_Cannon_BP.Incendiary_Cannon_BP_C" _returnvalue "Undefined" 0 0))
    (Actor|DestroyActor (Variables|Default|GetEquippedGun))
    (bind _output_get_2 (Variables|Default|SetEquippedGun _returnvalue_2))
    (Transformation|AttachComponentToComponent _output_get_2 (Variables|Default|GetGunLocation) "None" "SnapToTarget" "SnapToTarget" "KeepRelative" true)
    (elif (Utilities|ClassIsChildOf (Utilities|GetClass _output_get) "/Game/Tank/Power-Ups/Explosive_Power_Up_BP.Explosive_Power_Up_BP_C")
      (bind _returnvalue_3 (Game|SpawnActorfromClass "/Game/Tank/Explosive_Cannon_BP.Explosive_Cannon_BP_C" _returnvalue "Undefined" 0 0))
      (Actor|DestroyActor (Variables|Default|GetEquippedGun))
      (bind _output_get_3 (Variables|Default|SetEquippedGun _returnvalue_3))
      (Transformation|AttachComponentToComponent _output_get_3 (Variables|Default|GetGunLocation) "None" "SnapToTarget" "SnapToTarget" "KeepRelative" true)
      (elif (Utilities|ClassIsChildOf (Utilities|GetClass _output_get) "/Game/Tank/Power-Ups/Sniper_Power_Up_BP.Sniper_Power_Up_BP_C")
        (bind _returnvalue_4 (Game|SpawnActorfromClass "/Game/Tank/Sniper_Cannon_BP.Sniper_Cannon_BP_C" _returnvalue "Undefined" 0 0))
        (Actor|DestroyActor (Variables|Default|GetEquippedGun))
        (bind _output_get_4 (Variables|Default|SetEquippedGun _returnvalue_4))
        (Transformation|AttachComponentToComponent _output_get_4 (Variables|Default|GetGunLocation) "None" "SnapToTarget" "SnapToTarget" "KeepRelative" true)))))

(event Input|ActionEvents|InputActionFire
  (params (Key :type Key%20Structure :default "None"))
  ;[1 1 1] Fires projectile in arch
  (:Pressed
    (if (Variables|Default|GetCanShoot)
      (bind _returnvalue (Game|SpawnActorfromClass "/Game/Tank/Tank_Projectile_BP.Tank_Projectile_BP_C" (Math|Transform|MakeTransform (Transformation|GetWorldLocation (Variables|Default|GetBullet%20Spawn)) (Pawn|GetControlRotation :!class /Script/Engine.Pawn)) "Undefined" 0 0))
      (Game|Components|ProjectileMovement|SetVelocityinLocalSpace (Variables|/Game/Tank/Tank_Projectile_BP.Tank_Projectile_BP_C|GetProjectileMovement _returnvalue) (Variables|Default|GetInitial%20Local%20Velocity))
      (Transformation|SetActorScale3D _returnvalue (Math|Vector|MakeVector 2.0 2.0 2.0))
      (Variables|Default|SetCanShoot false)
      (Utilities|FlowControl|Delay (Variables|/Game/Tank/BaseGun_BP.BaseGun_BP_C|GetFireRate (Variables|Default|GetEquippedGun)))
      (Variables|Default|SetCanShoot true))))

(event Input|AxisEvents|InputAxisMoveForward
  (params (AxisValue :type Float%20%28single-precision%29))
  ;[1 1 1] Movemnet
  (if (not (Variables|Default|GetDisableMovement))
    (Pawn|Input|AddMovementInput (Math|Vector|GetForwardVector (Math|Rotator|MakeRotator 0.0 0.0 (.Yaw (Math|Rotator|BreakRotator (Pawn|GetControlRotation :!class /Script/Engine.Pawn))))) AxisValue false)))

(event Input|AxisEvents|InputAxisMoveRight
  (params (AxisValue :type Float%20%28single-precision%29))
  ;[1 1 1] Movemnet
)

(event Input|AxisEvents|InputAxisTurn
  (params (AxisValue :type Float%20%28single-precision%29))
  ;[1 1 1] Mouse
  (Pawn|Input|AddControllerYawInput AxisValue))

(event Input|AxisEvents|InputAxisLookUp
  (params (AxisValue :type Float%20%28single-precision%29))
  ;[1 1 1] Mouse
  (Pawn|Input|AddControllerPitchInput AxisValue))

(event Input|MouseEvents|LeftMouseButton
  (params (Key :type Key%20Structure :default "None"))
  ;[1 1 1] Gun shoot with left mouse click (Disabled)
)

(fn ConstructionScript)